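; BP_Grenade is an explosive projectile actor that is launched by an Ignite event and explodes on impact.
; Ignite detaches it from its parent, adds a projectile movement component at runtime with velocity along the fire direction, and enables collision on the Grenade component.
; A hit on any actor other than its owner spawns a Niagara explosion, applies radial damage with falloff, and destroys the grenade.
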(event OnComponentHit(Grenade)
  (params (HitComponent :type Primitive%20Component%20Object%20Reference) (OtherActor :type Actor%20Object%20Reference) (OtherComp :type Primitive%20Component%20Object%20Reference) (NormalImpulse :type Vector :default "0, 0, 0") (Hit :type Hit%20Result%20Structure%20%28by%20ref%29))
  (if (!= OtherActor (Components|GetOwner))
    (Niagara|SpawnSystematLocation "/Game/MsvFx_Niagara_Explosion_Pack_01/Prefabs/Niagara_Explosion_03.Niagara_Explosion_03" (Transformation|GetActorLocation))
    (Class|GameplayStatics|ApplyRadialDamagewithFalloff (Variables|Default|GetExplosion%20Damage) 0.0 (Transformation|GetActorLocation) 0.0 (Variables|Default|GetDamage%20Range) 1.0 0 0 self 0 "ECC_Visibility")
    (Actor|DestroyActor)))

(event Custom|Ignite
  (params (FireDirection :type Vector))
  (Transformation|DetachFromActor "KeepWorld" "KeepWorld" "KeepWorld")
  (bind _returnvalue (AddComponent|AddProjectileMovementComponent))
  (Variables|/Script/Engine.MovementComponent|SetVelocity _returnvalue (* FireDirection (Variables|Default|GetProjectileSpeed)))
  (Collision|SetCollisionEnabled (Variables|Default|GetGrenade) "QueryAndPhysics"))

(event EventBeginPlay)

(event Collision|EventActorBeginOverlap
  (params (OtherActor :type Actor%20Object%20Reference)))

(event EventTick
  (params (DeltaSeconds :type Float%20%28single-precision%29)))

(fn ConstructionScript)